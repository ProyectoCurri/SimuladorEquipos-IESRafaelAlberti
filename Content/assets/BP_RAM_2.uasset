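; BP_RAM_2 is a grabbable RAM stick that fits into the second RAM slot of the Placabase motherboard.
; On drop, a small sphere trace at its "join" socket checks for that board, then disables physics and snaps to socket "ram2" if RAM2Attached is false.
; Attaching sets that flag and fires the Attach dispatcher, while any grab clears it and fires Detach.
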(event `self.GrabComponent.OnDropped`
  (bind _placabase (`self.placabase`))
  (bind _returnvalue (`SceneComponent.GetSocketLocation` (`self.StaticMesh`) "join"))
  (bind (_outhit _returnvalue_2) (`KismetSystemLibrary.SphereTraceSingleForObjects` _returnvalue _returnvalue 10.0 (`|MakeArray` "ObjectTypeQuery4" :!type "EObjectTypeQuery Enum")))
  (if _returnvalue_2
    (bind (_bblockinghit _binitialoverlap _time _distance _location _impactpoint _normal _impactnormal _physmat _hitactor) (`GameplayStatics.BreakHitResult` _outhit))
    (if (== _placabase _hitactor)
      (if (not (`/Game/assets/BP_PlacaBase.RAM2Attached` _placabase))
        (`PrimitiveComponent.SetSimulatePhysics` (`self.StaticMesh`) false)
        (`self.K2_AttachToActor` _hitactor "ram2" "SnapToTarget" "SnapToTarget" "SnapToTarget" false)
        (set `/Game/assets/BP_PlacaBase.RAM2Attached` true _placabase)
        (`self.Attach`)))))

(event `self.GrabComponent.OnGrabbed`
  (set `/Game/assets/BP_PlacaBase.RAM2Attached` false (`self.placabase`))
  (`self.detach`))

(fn `UserConstructionScript`)