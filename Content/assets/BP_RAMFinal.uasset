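; Grabbable Corsair RGB RAM stick that snaps into the "ram" socket of its referenced Placabase (motherboard) actor.
; On drop, a small sphere trace at the mesh's "join" socket checks for that board with a free RAM slot.
; A match disables physics, attaches the stick, sets the board's RAMAttached flag and calls Attach.
; Grabbing clears the flag and calls Detach.
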(event `self.GrabComponent.OnDropped`
  (bind (_placabase _placabase_2) (`self.placabase`))
  (bind _returnvalue (`SceneComponent.GetSocketLocation` (`self.Corsair_RGB`) "join"))
  (bind (_outhit _returnvalue_2) (`KismetSystemLibrary.SphereTraceSingleForObjects` _returnvalue _returnvalue 10.0 (`|MakeArray` "ObjectTypeQuery4" :!type "EObjectTypeQuery Enum")))
  (if _returnvalue_2
    (bind (_bblockinghit _binitialoverlap _time _distance _location _impactpoint _normal _impactnormal _physmat _hitactor) (`GameplayStatics.BreakHitResult` _outhit))
    (if (== _placabase_2 _hitactor)
      (if (not (`/Game/assets/BP_PlacaBase.RAMAttached` _placabase_2))
        (`PrimitiveComponent.SetSimulatePhysics` (`self.Corsair_RGB`) false)
        (`self.K2_AttachToActor` _hitactor "ram" "SnapToTarget" "SnapToTarget" "SnapToTarget" false)
        (set `/Game/assets/BP_PlacaBase.RAMAttached` true _placabase_2)
        (`self.Attach`)))))

(event `self.GrabComponent.OnGrabbed`
  (set `/Game/assets/BP_PlacaBaseFinal.RAMAttached` false (`self.placabase`))
  (`self.detach`))

(fn `UserConstructionScript`)