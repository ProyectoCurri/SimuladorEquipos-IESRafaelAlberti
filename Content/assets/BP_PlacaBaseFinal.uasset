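; BP_PlacaBaseFinal is a motherboard Blueprint that tracks whether two RAM modules and a CPU are attached.
; Separate attachRAM, attachRAM2 and attachCPU events each set their own boolean flag if it is not already true.
; The allAttach event checks the three flags in nested branches but triggers nothing when all are set, and the construction script is empty.
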(event `allAttach`
  (if (`self.RAMAttached`)
    (if (`self.RAM2Attached`)
      (if (`self.CPUAttached`)
        _))))

(event `attachRAM2`
  (if (not (`self.RAM2Attached`))
    (set `self.RAM2Attached` true)))

(event `attachRAM`
  (if (not (`self.RAMAttached`))
    (set `self.RAMAttached` true)))

(event `attachCPU`
  (if (not (`self.CPUAttached`))
    (set `self.CPUAttached` true)))

(fn `UserConstructionScript`)