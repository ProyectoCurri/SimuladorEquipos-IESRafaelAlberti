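; BP_CPU is a grabbable CPU part that snaps onto a motherboard (Placabase) in what appears to be PC assembly gameplay.
; On drop, it sphere-traces physics bodies at its mesh socket and, if it hits that motherboard with no CPU attached, snaps to its socket.
; It then sets the motherboard's CPUAttached flag and calls Attach.
; Grabbing always clears the flag and calls Detach, even if the CPU was not attached.
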(event `self.GrabComponent.OnDropped`
  (bind _placabase (`self.placabase`))
  (bind _returnvalue (`SceneComponent.GetSocketLocation` (`self.procesador`) "Socket"))
  (bind (_outhit _returnvalue_2) (`KismetSystemLibrary.SphereTraceSingleForObjects` _returnvalue _returnvalue 10.0 (`|MakeArray` "ObjectTypeQuery4" :!type "EObjectTypeQuery Enum")))
  (if _returnvalue_2
    (bind (_bblockinghit _binitialoverlap _time _distance _location _impactpoint _normal _impactnormal _physmat _hitactor) (`GameplayStatics.BreakHitResult` _outhit))
    (if (== _placabase _hitactor)
      (if (not (`/Game/assets/BP_PlacaBase.CPUAttached` _placabase))
        (`self.K2_AttachToActor` _hitactor "Socket" "SnapToTarget" "SnapToTarget" "SnapToTarget" false)
        (set `/Game/assets/BP_PlacaBase.CPUAttached` true _placabase)
        (`self.Attach`)))))

(event `self.GrabComponent.OnGrabbed`
  (set `/Game/assets/BP_PlacaBase.CPUAttached` false (`self.placabase`))
  (`self.detach`))

(fn `UserConstructionScript`)